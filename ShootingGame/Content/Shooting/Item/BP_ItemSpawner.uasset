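; Item spawner actor that places a random item class from its Actor array at its own transform, on authority only.
; DoRandomItemSpawn binds to the spawned actor's destruction and sets a five-second timer if spawning fails, without a function name.
; The destroy handler sets a DoRandomItemSpawn timer, but targets the destroyed actor instead of the spawner.
; DT_Item lookups are disconnected, and nothing here starts the first spawn.
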(event EventBeginPlay)

(event Collision|EventActorBeginOverlap
  (params (OtherActor :type Actor%20Object%20Reference)))

(event EventTick
  (params (DeltaSeconds :type Float%20%28single-precision%29)))

(fn ConstructionScript)

(fn DoRandomItemSpawn
  (Networking|SwitchHasAuthority
    (:Authority
      (bind _returnvalue (Game|SpawnActorfromClass (.OutItem (Utilities|Array|Random (Variables|Default|GetActor))) (Transformation|GetActorTransform) "Undefined" "MultiplyWithRoot" 0 0))
      (Utilities|IsValid _returnvalue
        (:Is%20Valid
          ;[0.15 0.15 0.15 0.5] 디스트로이 이벤트 불러서  다시 스폰
          (Game|BindEventtoOnDestroyed _returnvalue (EventDispatchers|CreateEvent :!event EVItemDestroy)))
        (:Is%20Not%20Valid
          (Utilities|Time|SetTimerbyFunctionName 0 "" 5.0))))))

(fn EVItemDestroy
  (params (DestroyedActor :type Actor%20Object%20Reference))
  (Utilities|Time|SetTimerbyFunctionName DestroyedActor "DoRandomItemSpawn" 5.0))