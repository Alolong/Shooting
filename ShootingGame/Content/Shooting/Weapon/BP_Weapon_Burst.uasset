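; BP_Weapon_Burst is a weapon Blueprint that fires a burst of up to three shots per trigger press.
; EVOnTrigger resets the shot counter and starts a looping DoTrigger timer, ignoring presses while that timer exists.
; Each DoTrigger tick checks CanShoot, calls the parent's DoTrigger to shoot, and clears the timer at the shot limit or when shooting is not possible.
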(event EventBeginPlay
  (|CallParentFunction) ; This node is disabled and will not be called.\nDrag off pins to build functionality.
)

(event Collision|EventActorBeginOverlap
  (params (OtherActor :type Actor%20Object%20Reference))
  (|CallParentFunction OtherActor) ; This node is disabled and will not be called.\nDrag off pins to build functionality.
)

(event EventTick
  (params (DeltaSeconds :type Float%20%28single-precision%29))
  (|CallParentFunction DeltaSeconds) ; This node is disabled and will not be called.\nDrag off pins to build functionality.
)

(fn ConstructionScript
  (|CallParentFunction))

(fn EVonTrigger
  (params (isPress :type Boolean))
  (if isPress
    (if (not (Class|KismetSystemLibrary|TimerExists 0 "DoTrigger"))
      (Variables|Default|SetShootCnt 0)
      (Utilities|Time|SetTimerbyFunctionName 0 "DoTrigger" 0.1 true)
      (return false))))

(fn DoTrigger
  (if (CallFunction|CanShoot)
    (|CallParentFunction)
    ;[0.15 0.15 0.15 0.5] 3발 이상 시 반복취소
    (bind _output_get (Variables|Default|SetShootCnt (+ (Variables|Default|GetShootCnt) 1)))
    (if (>= _output_get 3)
      (Utilities|Time|ClearTimerbyFunctionName 0 "DoTrigger"))
    (else
      (Utilities|Time|ClearTimerbyFunctionName 0 "DoTrigger"))))