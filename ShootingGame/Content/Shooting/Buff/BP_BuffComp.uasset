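; Buff component that grants timed buffs from DT_Buff to its owner; invincibility is the only type handled here.
; AddBuff ignores active duplicates, records the row, then sets the Invincible flag and attaches a Niagara effect to the Character mesh.
; UpdateBuffTick advances timers, then removes expired buffs one per pass, rescanning until none remain to avoid mutating the array mid-iteration.
; Removal clears the flag and destroys the effect stored by row name.
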(event EventBeginPlay)

(event EventTick
  (params (DeltaSeconds :type Float%20%28single-precision%29)))

(fn AddBuff
  (params (RowName :type Name))
  (if (not (CallFunction|IsApplyBuff RowName))
    (bind _returnvalue (Utilities|GetDataTableRow "/Game/Shooting/Buff/DT_Buff.DT_Buff" RowName)
      (:then
        (Utilities|Array|Add (Variables|Default|GetBuffRef) (Utilities|Struct|MakeST_BuffRef _returnvalue 0.0 RowName))
        (CallFunction|EvApplyBuff RowName)))))

(fn UpdateBuffTick
  (params (Deltaseconds :type Float%20%28double-precision%29))
  (Utilities|FlowControl|Sequence
    (:then_0
      (CallFunction|UpdateBuffTime Deltaseconds))
    (:then_1
      ;[0.15 0.15 0.15 0.5] True가 나올 때까지 계속 돌림
      (bind _iscompleted (CallFunction|UpdateBuffTimeOver :!label _label))
      (if (not _iscompleted)
        (goto _label)))))

(fn UpdateBuffTime
  (params (DeltaSeconds :type Float%20%28double-precision%29))
  ;[0.15 0.15 0.15 0.5] 시간을 계속 업데이트
  (for (_ _array_index) (Variables|Default|GetBuffRef)
    (Utilities|Struct|SetmembersinST_BuffRef (Utilities|Array|Get(acopy) (Variables|Default|GetBuffRef) _array_index) (+ (.Cur_Duration (Utilities|Struct|BreakST_BuffRef (Utilities|Array|Get(acopy) (Variables|Default|GetBuffRef) _array_index))) (LocalVariables|GetDeltaseconds))) ; Detils에서 cur duration 연결
  ))

(fn UpdateBuffTimeOver
  ;[0.15 0.15 0.15 0.5] Update Buff Time Over
  (for (_array_element _array_index) (Variables|Default|GetBuffRef)
    (if (<= (.duration (.BuffData (Utilities|Struct|BreakST_BuffRef _array_element))) (.Cur_Duration (Utilities|Struct|BreakST_BuffRef _array_element)))
      (CallFunction|EvRemoveBuff (.RowName (Utilities|Struct|BreakST_BuffRef _array_element)))
      (Utilities|Array|RemoveIndex (Variables|Default|GetBuffRef) _array_index)
      (return false)))
  (return true))

(fn EvApplyBuff
  (params (RowName :type Name))
  (bind _returnvalue (Utilities|GetDataTableRow "/Game/Shooting/Buff/DT_Buff.DT_Buff" RowName)
    (:then
      (switch Utilities|FlowControl|Switch|SwitchonEn_BuffType (.bufftype _returnvalue)
        (:NewEnumerator1
          (Variables|Default|SetInvincible true)
          (bind _ascharacter (Utilities|Casting|CastToCharacter (Components|GetOwner)))
          (bind _returnvalue_2 (Niagara|SpawnSystemAttached "/Game/Basic_VFX/Niagara/NS_Basic_9.NS_Basic_9" (Variables|/Script/Engine.Character|GetMesh _ascharacter) "None" "0.000000,0.000000,30.000000" "0, 0, 0" "KeepRelativeOffset" false))
          (Niagara|SetNiagaraVariable(Float) _returnvalue_2 "ParticleSize" 3e+01)
          ;[0.15 0.15 0.15 0.5] RowName으로 저장이 됨
          (Utilities|Map|Add (Variables|Default|GetInvincibleEffect) RowName _returnvalue_2))))))

(fn EvRemoveBuff
  (params (RowName :type Name))
  (bind _returnvalue (Utilities|GetDataTableRow "/Game/Shooting/Buff/DT_Buff.DT_Buff" RowName)
    (:then
      (switch Utilities|FlowControl|Switch|SwitchonEn_BuffType (.bufftype _returnvalue)
        (:NewEnumerator1
          (Variables|Default|SetInvincible false)
          (Components|DestroyComponent (.Value (Utilities|Map|Find (Variables|Default|GetInvincibleEffect) RowName)))
          (Utilities|Map|Remove (Variables|Default|GetInvincibleEffect) RowName))))))

(fn IsInvincible
  (return (Variables|Default|GetInvincible)))

(fn IsApplyBuff
  (params (RowName :type Name))
  (for _array_element (Variables|Default|GetBuffRef)
    (if (== (.RowName (Utilities|Struct|BreakST_BuffRef _array_element)) RowName)
      (return true)))
  (return false))