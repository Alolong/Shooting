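; Lobby HUD actor that creates the lobby widget on BeginPlay and keeps its player list up to date.
; BindPS hooks a lobby PlayerState's nickname-change and destroyed events and triggers an immediate refresh.
; Refreshes go through UpdateChangeNickName, which updates the widget's list view or retries on a short timer until the widget is valid.
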(event EventBeginPlay
  (bind _returnvalue (UserInterface|CreateWidget "/Game/Widget/Lobby/Lobbi_hud_widget.Lobbi_hud_widget_C"))
  (bind _output_get (Variables|Default|SetLobbyHud _returnvalue))
  (UserInterface|Viewport|AddtoViewport _output_get 0))

(event Collision|EventActorBeginOverlap
  (params (OtherActor :type Actor%20Object%20Reference)))

(event EventTick
  (params (DeltaSeconds :type Float%20%28single-precision%29)))

(fn ConstructionScript)

(fn BindPS
  (params (LobbyPS :type BP%20Lobby%20PS%20Object%20Reference))
  (EventDispatchers|BindEventtoDSChangeNickname LobbyPS (EventDispatchers|CreateEvent :!event EVChangeNickName))
  (CallFunction|EVChangeNickName (Variables|/Game/GMB/lobby/BP_LobbyPS.BP_LobbyPS_C|GetNickName LobbyPS))
  (Game|BindEventtoOnDestroyed LobbyPS (EventDispatchers|CreateEvent :!event EVDestroyPS)))

(fn EVChangeNickName
  (params (NickNameToChange :type String))
  (CallFunction|UpdateChangeNickName))

(fn UpdateChangeNickName
  (bind _lobbyhud (Variables|Default|GetLobbyHud)
    (:then
      (Default|UpdatePlayerListview _lobbyhud))
    (:else
      (Utilities|Time|SetTimerbyFunctionName 0 "UpdateChangeNickName" 0.01))))

(fn EVDestroyPS
  (params (DestroyedActor :type Actor%20Object%20Reference))
  (CallFunction|UpdateChangeNickName))