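; BP_Bomb is a bomb actor that damages a shooting character on contact and then destroys itself.
; Its Sphere overlap runs on authority only, casting to BP_ShootingChar and calling AddDMG on that character's BP_PlayerState with a fixed amount.
; A separate DoDMG function, not called in this graph, ignores its HP inputs and adds zero damage to player 0's state.
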(event OnComponentBeginOverlap(Sphere)
  (params (OverlappedComponent :type Primitive%20Component%20Object%20Reference) (OtherActor :type Actor%20Object%20Reference) (OtherComp :type Primitive%20Component%20Object%20Reference) (OtherBodyIndex :type Integer) (bFromSweep :type Boolean) (SweepResult :type Hit%20Result%20Structure%20%28by%20ref%29))
  (Networking|SwitchHasAuthority
    (:Authority
      (bind _asbp_shooting_char (Utilities|Casting|CastToBP_ShootingChar OtherActor))
      (bind _asbp_player_state (Utilities|Casting|CastToBP_PlayerState (Variables|/Script/Engine.Pawn|GetPlayerState _asbp_shooting_char)))
      (Default|AddDMG _asbp_player_state 1e+01)
      (CallFunction|Destroyself))))

(event EventBeginPlay)

(event Collision|EventActorBeginOverlap
  (params (OtherActor :type Actor%20Object%20Reference)))

(event EventTick
  (params (DeltaSeconds :type Float%20%28single-precision%29)))

(fn ConstructionScript)

(fn DoDMG
  (params (CurHP :type Float%20%28double-precision%29) (MaxHP :type Float%20%28double-precision%29))
  (bind _asbp_player_state (Utilities|Casting|CastToBP_PlayerState (Game|GetPlayerState 0)))
  (Default|AddDMG _asbp_player_state 0.0))

(fn Destroyself
  (Actor|DestroyActor))