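; Networked weapon actor that attaches to a character's weapon socket or detaches with physics, configured by weapon data.
; Trigger and reload play montages; EVFire spawns muzzle effects, and the local player sends a camera-based shot to ReqFire for server tracing and damage.
; Reload completion requests a magazine from PlayerState to refill ammo.
; Ammo replication updates the owner's HUD, while BP_BuffComp can grant infinite ammo or block shooting during invincibility.
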(event Custom|ReqFire
  (params (StartLoc :type Vector) (EndLoc :type Vector))
  ;[0.15 0 0 0.5] 서버-발사
  (CallFunction|UseAmmo)
  ;;[0.15 0.15 0.15 0.5] 발사 궤적 처리
  (bind _outhit (Collision|LineTraceForObjects StartLoc EndLoc (Utilities|Array|MakeArray "ObjectTypeQuery1" "ObjectTypeQuery2" "ObjectTypeQuery3" "ObjectTypeQuery4" "ObjectTypeQuery6") false (Utilities|Array|MakeArray (Variables|Default|GetCharacter)) "ForDuration" true "(R=1.000000,G=0.000000,B=0.000000,A=1.000000)" "(R=0.000000,G=1.000000,B=0.000000,A=1.000000)" 1e+01))
  ;;[0.15 0.15 0.15 0.5] 데미지 처리
  (Game|Damage|ApplyDamage (.HitActor (Collision|BreakHitResult _outhit)) (.damage (Variables|Default|GetWeponData)) (Pawn|GetController (Variables|Default|GetCharacter)) self))

(event Custom|ReqReload
  ;[0.15 0 0 0.5] 서버-리로드
  (bind _character (Variables|Default|GetCharacter)
    (:then
      (bind _asbp_player_state (Utilities|Casting|CastToBP_PlayerState (Variables|/Script/Engine.Pawn|GetPlayerState _character)))
      (bind _isused (Default|UseMag _asbp_player_state))
      (if _isused
        (Variables|Default|SetAmmo (.maxammo (Variables|Default|GetWeponData)))))
    (:else)))

(event EventBeginPlay
  (bind _wepondata (Variables|Default|GetWeponData))
  (Variables|Default|SetAmmo (.maxammo _wepondata))
  (Components|StaticMesh|SetStaticMesh (Variables|Default|GetWeapone) (.mesh _wepondata)))

(fn ConstructionScript)

(fn GetNearestWeapon
  (return 0))

(fn DoReload
  (bind _character (Variables|Default|GetCharacter)
    (:then
      (Animation|PlayAnimMontage _character (.reloadmontage (Variables|Default|GetWeponData)) 1.0 "None"))
    (:else)))

(fn DoTrigger
  ;[0.15 0.15 0.15 0.5] 예외처리
  (bind _character (Variables|Default|GetCharacter)
    (:then
      (Animation|PlayAnimMontage _character (.shootmontage (Variables|Default|GetWeponData)) 1.0 "None"))
    (:else)))

(fn HasOwner
  (return (Utilities|IsValid (Variables|Default|GetCharacter))))

(fn FireEffect
  (bind _weapone (Variables|Default|GetWeapone))
  (bind _returnvalue (Transformation|GetSocketTransform _weapone "Muzzle" "RTS_World"))
  (Effects|SpawnEmitteratLocation "/Game/StarterContent/Particles/P_Explosion.P_Explosion" (.location _returnvalue) (.rotation _returnvalue) "0.100000,0.100000,0.100000")
  (Audio|SpawnSoundatLocation "/Game/StarterContent/Audio/Explosion_Cue.Explosion_Cue" (.location _returnvalue) "0, 0, 0" 1.0 1.0 0.0 0 0))

(fn EVMontageEnd
  (params (Montage :type Anim%20Montage%20Object%20Reference) (bInterrupted :type Boolean)))

(fn UseAmmo
  ;[0.15 0 0 0.5] 서버
  (if (CallFunction|CanShoot)
    (Variables|Default|SetAmmo (Math|Integer|Clamp(Integer) (- (Variables|Default|GetAmmo) 1) 0 (.maxammo (Variables|Default|GetWeponData))))
    (return true)
    (else
      (return false))))

(fn UpdateAmmoUI
  (params (Ammo :type Integer))
  (if (== (Variables|Default|GetCharacter) (Pawn|GetControlledPawn (Game|GetPlayerController 0)))
    (bind _asbp_hud (Utilities|Casting|CastToBP_Hud (HUD|GetHUD (Game|GetPlayerController 0))))
    (Default|UpdateAmmo _asbp_hud Ammo)))

(fn OnRepAmmo
  ;[0.15 0.15 0.15 0.5] 클라
  (CallFunction|UpdateAmmoUI (Variables|Default|GetAmmo)))

(fn CanShoot
  (bind _character (Variables|Default|GetCharacter))
  (bind _returnvalue (Actor|GetComponentbyClass _character "/Game/GMB/Shooting/Buff/BP_BuffComp.BP_BuffComp_C"))
  (Utilities|IsValid _returnvalue
    (:Is%20Valid
      (return (or (Default|IsInfiniteAmmo _returnvalue) (and (not (Default|IsInvincible _returnvalue)) (> (Variables|Default|GetAmmo) 0)))))
    (:Is%20Not%20Valid
      (return (> (Variables|Default|GetAmmo) 0)))))

(fn EVDoReload
  (bind _character (Variables|Default|GetCharacter)
    (:then
      (Animation|PlayAnimMontage _character (.reloadmontage (Variables|Default|GetWeponData)) 1.0 "None"))
    (:else)))

(fn EVReloadComplete
  (Utilities|IsOwnChar
    (:True
      (CallFunction|ReqReload)
      (return false))))

(fn EVAttachtoChar
  (params (Character :type Character%20Object%20Reference))
  ;[0.15 0.15 0.15 0.5] 변수로 저장된 캐릭터
  (bind _output_get (Variables|Default|SetCharacter Character))
  (Physics|SetSimulatePhysics (Variables|Default|GetWeapone) false)
  (EventDispatchers|BindEventtoOnMontageEnded (Components|SkeletalMesh|GetAnimInstance (Variables|/Script/Engine.Character|GetMesh _output_get)) (EventDispatchers|CreateEvent :!event EVMontageEnd))
  (bind _returnvalue (Transformation|AttachComponentToComponent (Variables|/Script/Engine.Character|GetMesh _output_get) "Weapon" "SnapToTarget" "SnapToTarget" "KeepWorld" true))
  (CallFunction|UpdateAmmoUI (Variables|Default|GetAmmo))
  (return _returnvalue))

(fn EVDetachfromChar
  (params (Character :type Character%20Object%20Reference))
  (Transformation|DetachFromComponent (Variables|Default|GetWeapone) "KeepWorld" "KeepWorld" "KeepRelative" true)
  (Physics|SetSimulatePhysics (Variables|Default|GetWeapone) true)
  ;[0.15 0.15 0.15 0.5] 몽타주 끝날 시 발생 이벤트
  (bind _character (Variables|Default|GetCharacter)
    (:then
      (EventDispatchers|UnbindEventfromOnMontageEnded (Components|SkeletalMesh|GetAnimInstance (Variables|/Script/Engine.Character|GetMesh _character)) (EventDispatchers|CreateEvent :!event EVMontageEnd))
      (CallFunction|UpdateAmmoUI)
      ;[0.15 0.15 0.15 0.5] 캐릭터 값을 비워주는 역할
      (Variables|Default|SetCharacter 0)
      (return false))
    (:else)))

(fn EVFire
  (bind _returnvalue (Game|GetPlayerCameraManager 0))
  (bind _returnvalue_2 (Transformation|GetActorLocation _returnvalue))
  (CallFunction|FireEffect)
  ;[0.15 0.15 0.15 0.5] 지금 플레이어가 0번 플레이어랑 같은지 판단 클라
  (if (== (Pawn|GetController (Variables|Default|GetCharacter)) (Game|GetPlayerController 0))
    ;[0.15 0.15 0.15 0.5] 서버로
    (CallFunction|ReqFire _returnvalue_2 (+ _returnvalue_2 (* (Transformation|GetActorForwardVector _returnvalue) 1e+05)))
    (return false)))

(fn EVIsReloading
  ;[0.15 0.15 0.15 0.5] 장착한 캐릭터의 애니몽타주에 접근하여 데이터의 애니와 동일한지 검사
  (bind _character (Variables|Default|GetCharacter)
    (:then
      (return (== (.reloadmontage (Variables|Default|GetWeponData)) (Animation|Montage|GetCurrentActiveMontage (Components|SkeletalMesh|GetAnimInstance (Variables|/Script/Engine.Character|GetMesh _character))))))
    (:else)))

(fn EVonTrigger
  (params (isPress :type Boolean))
  (if isPress
    (CallFunction|DoTrigger)
    (return false)))

(fn EVTrigger
  (params (IsPress :type Boolean))
  ;[0.15 0.15 0.15 0.5] 총기애니- 각각 애니 다름
  (if IsPress
    (CallFunction|DoTrigger)
    (return false)))

(fn IsCanShoot
  (return (CallFunction|CanShoot)))