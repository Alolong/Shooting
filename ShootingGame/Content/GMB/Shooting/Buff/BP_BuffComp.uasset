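; Buff component for a Character that grants timed buffs from DT_Buff, currently invincibility and infinite ammo, each with an attached Niagara effect.
; AddBuff ignores duplicates, records the buff in BuffRef and BuffPackets, then sets its flag and effect.
; Tick advances timers and drops expired buffs, with only the authority firing ResRemoveBuff to clear flag and effect.
; Clients replay BuffPackets through AddBuff on BeginPlay to show existing buffs.
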(event Custom|ResRemoveBuff
  (params (RowName :type Name))
  (CallFunction|EvRemoveBuff RowName))

(event EventBeginPlay
  ;[0.15 0.15 0.15 0.5] 클라에서 실행
  (Networking|SwitchHasAuthority
    (:Remote
      ;[0.15 0.15 0.15 0.5] 클라에서 버프 보이게
      (for _array_element (Variables|Default|GetBuffPackets)
        ;;[0.15 0.15 0.15 0.5] 시각적으로 처리
        (CallFunction|AddBuff (.BuffRowName (Utilities|Struct|BreakST_BuffPacket _array_element)) (.CurDuration (Utilities|Struct|BreakST_BuffPacket _array_element)))))))

(event EventTick
  (params (DeltaSeconds :type Float%20%28single-precision%29))
  (CallFunction|UpdateBuffTick DeltaSeconds))

(fn AddBuff
  (params (RowName :type Name) (CurDuration :type Float%20%28double-precision%29))
  ;[0.15 0.15 0.15 0.5] 현재 적용중인 버프인지 체크(Pure한 함수)
  (if (not (CallFunction|IsApplyBuff RowName))
    (bind _returnvalue (Utilities|GetDataTableRow "/Game/GMB/Shooting/Buff/DT_Buff.DT_Buff" RowName)
      (:then
        ;[0.15 0.15 0.15 0.5] 버프 이름만 담음
        (Utilities|Array|Add (Variables|Default|GetBuffRef) (Utilities|Struct|MakeST_BuffRef _returnvalue 0.0 RowName))
        ;[0.15 0.15 0.15 0.5] 버프 패킷(서버->클라)
        ; 버프 이름, 시간값 담음
        (Utilities|Array|Add (Variables|Default|GetBuffPackets) (Utilities|Struct|MakeST_BuffPacket RowName CurDuration))
        ;[0.15 0.15 0.15 0.5] 버프 적용
        (CallFunction|EvApplyBuff RowName)))))

(fn EvApplyBuff
  (params (RowName :type Name))
  (bind _returnvalue (Utilities|GetDataTableRow "/Game/GMB/Shooting/Buff/DT_Buff.DT_Buff" RowName)
    (:then
      ;[0.15 0.15 0.15 0.5] 버프(실제적용)과 보이는 효과 나누기
      (Utilities|FlowControl|Sequence
        (:then_0
          ;[0.15 0.15 0.15 0.5] 실제 수치상 버프의 ON 체크
          (switch Utilities|FlowControl|Switch|SwitchonEn_BuffType (.Bufftype (Utilities|Struct|BreakST_Buff _returnvalue))
            (:NewEnumerator1
              (Variables|Default|SetInvincible true))
            (:NewEnumerator2
              (Variables|Default|SetInfiniteAmmo true))))
        (:then_1
          ;[0.15 0.15 0.15 0.5] 이펙트의 처리
          (CallFunction|ApplyEffect (.Naiagara (Utilities|Struct|BreakST_Buff _returnvalue)) RowName))))))

(fn IsApplyBuff
  (params (RowName :type Name))
  ;[0.15 0.15 0.15 0.5] 버프명 갖고옴
  (for _array_element (Variables|Default|GetBuffRef)
    ;[0.15 0.15 0.15 0.5] 데이터테이블과 비교하여 같은지 체크
    (if (== (.RowName (Utilities|Struct|BreakST_BuffRef _array_element)) RowName)
      (return true)))
  (return false))

(fn UpdateBuffTick
  (params (Deltaseconds :type Float%20%28double-precision%29))
  (Utilities|FlowControl|Sequence
    (:then_0
      (CallFunction|UpdateBuffTime Deltaseconds))
    (:then_1
      ;[0.15 0.15 0.15 0.5] True가 나올 때까지 계속 돌림
      (bind _iscompleted (CallFunction|UpdateBuffTimeOver :!label _label))
      (if (not _iscompleted)
        (goto _label)))))

(fn UpdateBuffTime
  (params (DeltaSeconds :type Float%20%28double-precision%29))
  ;[0.15 0.15 0.15 0.5] 시간을 계속 업데이트
  (for (_ _array_index) (Variables|Default|GetBuffRef)
    (Utilities|Struct|SetmembersinST_BuffRef (Utilities|Array|Get(acopy) (Variables|Default|GetBuffRef) _array_index) (+ (.Cur_Duration (Utilities|Struct|BreakST_BuffRef (Utilities|Array|Get(acopy) (Variables|Default|GetBuffRef) _array_index))) (LocalVariables|GetDeltaseconds))) ; Detils에서 cur duration 연결
  ))

(fn UpdateBuffTimeOver
  ;[0.15 0.15 0.15 0.5] 배열상 버프 진행 기간 비교
  (for (_array_element _array_index) (Variables|Default|GetBuffRef)
    (if (<= (.duration (.BuffData (Utilities|Struct|BreakST_BuffRef _array_element))) (.Cur_Duration (Utilities|Struct|BreakST_BuffRef _array_element)))
      (Networking|SwitchHasAuthority
        (:Authority
          ;[0.15 0.15 0.15 0.5] 이벤트 그래프에서
          ; 리스폰(서버->클라) 할 이벤트
          ; RemoveBuff와 연결되어 있다.
          (CallFunction|ResRemoveBuff (.RowName (Utilities|Struct|BreakST_BuffRef _array_element)) :!pinned true) ; 서버
        )
        (:Remote
          _))
      (Utilities|Array|RemoveIndex (Variables|Default|GetBuffRef) _array_index :!pinned true) ; 이 뒤는 서버,클라모두해당
      (Utilities|Array|RemoveIndex (Variables|Default|GetBuffPackets) _array_index)
      (return false)))
  (return true))

(fn EvRemoveBuff
  (params (RowName :type Name))
  (bind _returnvalue (Utilities|GetDataTableRow "/Game/GMB/Shooting/Buff/DT_Buff.DT_Buff" RowName)
    (:then
      (Utilities|FlowControl|Sequence
        (:then_0
          (switch Utilities|FlowControl|Switch|SwitchonEn_BuffType (.bufftype _returnvalue)
            (:NewEnumerator1
              (Variables|Default|SetInvincible false))
            (:NewEnumerator2
              (Variables|Default|SetInfiniteAmmo false))))
        (:then_1
          (CallFunction|RemoveEffect RowName))))))

(fn MakeBuffData
  (for _array_element (Variables|Default|GetBuffRef)
    ;[0.15 0.15 0.15 0.5] 배열에 추가
    (Utilities|Array|Add (LocalVariables|GetBuffPaket) (Utilities|Struct|MakeST_BuffPacket (.RowName (Utilities|Struct|BreakST_BuffRef _array_element)) (.Cur_Duration (Utilities|Struct|BreakST_BuffRef _array_element)))))
  (return (LocalVariables|GetBuffPaket)))

(fn ApplyEffect
  (params (Niagara :type Niagara%20System%20Object%20Reference) (RowName :type Name))
  ;[0.15 0.15 0.15 0.5] 캐릭터 가져오기
  (bind _ascharacter (Utilities|Casting|CastToCharacter (Components|GetOwner)))
  ;[0.15 0.15 0.15 0.5] 캐릭터에 이펙트나이아가라 붙이기
  ;;[0.15 0.15 0.15 0.5] 붙일 위치
  (bind _returnvalue (Niagara|SpawnSystemAttached Niagara (Variables|/Script/Engine.Character|GetMesh _ascharacter) "None" "0.000000,0.000000,30.000000" "0, 0, 0" "KeepRelativeOffset" false))
  ;;[0.15 0.08494 0.03284 0.5] 나이아가라에서 만든 변수의 값 조정
  (Niagara|SetNiagaraVariable(Float) _returnvalue "" 3e+01)
  ;[0.15 0.15 0.15 0.5] RowName에 나이아가라가 저장이 됨
  ; 1.Name변수 생성
  ; 2.Maps버튼 누르고 나이아가라 파티클로
  ; 3.받아온 이름과 맞는 나이아가라 넣기
  (Utilities|Map|Add (Variables|Default|GetInvincibleEffect) RowName _returnvalue))

(fn RemoveEffect
  (params (RowName :type Name))
  (bind _invincibleeffect (Variables|Default|GetInvincibleEffect))
  (bind (_value _returnvalue) (Utilities|Map|Find _invincibleeffect RowName))
  ;[0.15 0.15 0.15 0.5] 이름에 맞는 컴포넌트(나이아가라)삭제
  (Components|DestroyComponent _value)
  (if _returnvalue
    ;[0.15 0.15 0.15 0.5] 동적할당 해제
    (Utilities|Map|Remove (Variables|Default|GetInvincibleEffect) RowName)))

(fn IsInvincible
  (return (Variables|Default|GetInvincible)))

(fn IsInfiniteAmmo
  (return (Variables|Default|GetInfiniteAmmo)))