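; Game mode Blueprint that drives match phases (Ready, Play, End) and assigns player results.
; On BeginPlay it binds to the game state's phase and time dispatchers, then sets Ready.
; It caches phase updates and switches Ready to Play once the reported time exceeds six seconds.
; OnGameEnd sets End, giving the passed character's PlayerState one result and the others another.
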(event EventBeginPlay
  (CallFunction|BindGS))

(event EventTick
  (params (DeltaSeconds :type Float%20%28single-precision%29)))

(fn ConstructionScript)

(fn BindGS
  (bind _asbp_gs (Utilities|Casting|CastTo (Game|GetGameState)))
  (EventDispatchers|BindEventtoDSUpdateGS _asbp_gs (EventDispatchers|CreateEvent :!event EVUpdateGS))
  (EventDispatchers|BindEventtoDSDeltaSec _asbp_gs (EventDispatchers|CreateEvent :!event EVUpdateTS))
  (bind _asbp_gs_2 (Utilities|Casting|CastTo (Game|GetGameState)))
  (CallFunction|ChangeGS _asbp_gs_2 "NewEnumerator1"))

(fn EVUpdateGS
  (params (NewParam :type EN_GS%20Enum :default "NewEnumerator0"))
  (Variables|Default|SetGS NewParam))

(fn EVUpdateTS
  (params (DeltaSec :type Float%20%28double-precision%29))
  (switch Utilities|FlowControl|Switch|SwitchonEN_GS (Variables|Default|GetGS)
    (:NewEnumerator1
      (if (> DeltaSec 6.0)
        (bind _asbp_gs (Utilities|Casting|CastTo (Game|GetGameState)))
        (CallFunction|ChangeGS _asbp_gs "NewEnumerator2")))))

(fn OnGameEnd
  (params (Char :type Character%20Object%20Reference))
  (bind _asbp_gs (Utilities|Casting|CastTo (Game|GetGameState)))
  (CallFunction|ChangeGS _asbp_gs "NewEnumerator3")
  (CallFunction|UpdatePlayerResult Char))

(fn UpdatePlayerResult
  (params (self2 :type Pawn%20Object%20Reference))
  (bind _asbp_ps (Utilities|Casting|CastTo (Variables|/Script/Engine.Pawn|GetPlayerState self2)))
  (CallFunction|SetResult _asbp_ps "NewEnumerator0")
  (bind _outactors (Actor|GetAllActorsOfClass 0))
  (for _array_element _outactors
    (if (!= _array_element _asbp_ps)
      (CallFunction|SetResult _array_element "NewEnumerator2"))))